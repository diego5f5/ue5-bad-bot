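; BP_SmallSphere is an actor that drifts through the world while spinning at a random rate.
; On BeginPlay it picks a random rotator, scaled by RotationScaleFactor, as its per-second rotation.
; Each Tick it moves along its forward vector at Speed, then applies that rotation, both scaled by delta time.
; Because movement follows the rotating forward vector, its path curves; movement does not sweep for collision.
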(event EventTick
  (params (DeltaSeconds :type Float%20%28single-precision%29))
  (CallFunction|UpdateLocation)
  (CallFunction|UpdateRotation))

(event EventBeginPlay
  (CallFunction|InitializeDeltaRotation))

(fn ConstructionScript)

(fn InitializeDeltaRotation
  (Variables|SphereMovement|SetDelta%20Rotation (* (Math|Random|RandomRotator false) (Variables|SphereMovement|GetRotationScaleFactor))))

(fn UpdateLocation
  (Transformation|AddActorWorldOffset (* (* (Utilities|Time|GetWorldDeltaSeconds) (Variables|SphereMovement|GetSpeed)) (Transformation|GetActorForwardVector))))

(fn UpdateRotation
  (Class|Actor|AddActorWorldRotation (* (Variables|SphereMovement|GetDelta%20Rotation) (Utilities|Time|GetWorldDeltaSeconds))))